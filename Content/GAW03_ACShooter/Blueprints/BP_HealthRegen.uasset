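; BP_HealthRegen is a health pickup that flies toward the player and restores health on contact.
; When the player pawn enters LootRange, the MoveTo timeline interpolates the pickup from its start location to the player's live location, with sweep.
; Sphere overlap passes the other actor to the ACRegen component's RegenHealth and destroys the pickup only on success.
; The construction script tints the sphere through a dynamic material's Color parameter.
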(event OnComponentBeginOverlap(LootRange)
  (params (OverlappedComponent :type Primitive%20Component%20Object%20Reference) (OtherActor :type Actor%20Object%20Reference) (OtherComp :type Primitive%20Component%20Object%20Reference) (OtherBodyIndex :type Integer) (bFromSweep :type Boolean) (SweepResult :type Hit%20Result%20Structure%20%28by%20ref%29))
  (bind _returnvalue (Game|Player|GetPlayerPawn 0))
  (bind _returnvalue_2 (Transformation|GetActorLocation _returnvalue))
  (if (== OtherActor _returnvalue)
    (Variables|Default|SetStartLocation (Transformation|GetActorLocation))
    (bind _percent (Timeline|MoveTo Play)
      (:Update
        (Transformation|SetActorLocation (- _returnvalue_2 (* (- _returnvalue_2 (Variables|Default|GetStartLocation)) _percent)) true false)))))

(event OnComponentBeginOverlap(Sphere)
  (params (OverlappedComponent :type Primitive%20Component%20Object%20Reference) (OtherActor :type Actor%20Object%20Reference) (OtherComp :type Primitive%20Component%20Object%20Reference) (OtherBodyIndex :type Integer) (bFromSweep :type Boolean) (SweepResult :type Hit%20Result%20Structure%20%28by%20ref%29))
  (bind _hassucceded (Default|RegenHealth (Variables|Default|GetAC_Regen) OtherActor))
  (if _hassucceded
    (Actor|DestroyActor)))

(fn ConstructionScript
  (bind _sphere (Variables|Default|GetSphere))
  (bind _returnvalue (Rendering|Material|CreateDynamicMaterialInstance _sphere 0 (Rendering|Material|GetMaterial _sphere 0) :!class /Script/Engine.PrimitiveComponent))
  (Rendering|Material|SetVectorParameterValue _returnvalue "Color" (Variables|Default|GetColor) :!class /Script/Engine.MaterialInstanceDynamic))