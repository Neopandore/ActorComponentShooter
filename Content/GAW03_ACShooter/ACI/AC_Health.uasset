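; AC_Health is an actor component that tracks health for its owning actor, starting at maximum on BeginPlay.
; The IDamages event subtracts health, then CheckIfDead fires FireDeath at zero or below, which sends IDeathMessage to the owner.
; The IRegen event adds health up to the maximum and is ignored once health is depleted.
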(event Custom|FireDeath
  (Class|IHealth|IDeath(Message) (Variables|Default|GetAttachedActor)))

(event EventIDamages
  (params (DamageValue :type Integer))
  (Variables|Default|SetHealth_Current (- (Variables|Default|GetHealth_Current) DamageValue))
  (CallFunction|CheckifDead) ; FireDeath if true
)

(event EventIRegen
  (params (RegenValue :type Integer))
  (bind _health_max (Variables|Default|GetHealth_Max))
  (if (not (<= (Variables|Default|GetHealth_Current) 0))
    (if (>= (+ (Variables|Default|GetHealth_Current) RegenValue) _health_max)
      (Variables|Default|SetHealth_Current _health_max)
      (else
        (Variables|Default|SetHealth_Current (+ (Variables|Default|GetHealth_Current) RegenValue))))))

(event EventBeginPlay
  (Variables|Default|SetAttachedActor (Components|GetOwner))
  (Variables|Default|SetHealth_Current (Variables|Default|GetHealth_Max)))

(fn CheckifDead
  (if (<= (Variables|Default|GetHealth_Current) 0)
    (CallFunction|FireDeath)))